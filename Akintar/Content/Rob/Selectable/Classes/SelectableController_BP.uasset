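; SelectableController_BP is a selectable unit that moves by AI to a clicked location.
; Cursor-over events on its static mesh swap between highlight and base materials while it is unselected.
; Select and Deselect events track the selection flag and set the matching material.
; RightClick passes the hit location to AIMoveTo on itself and prints debug text on success or failure, without checking selection.
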(event OnBeginCursorOver(StaticMesh)
  (params (TouchedComponent :type Primitive%20Component%20Object%20Reference))
  (if (not (Variables|Default|GetisSelected))
    (Rendering|Material|SetMaterial (Variables|Default|GetStaticMesh) 0 (Variables|Default|GetmatHighlight))))

(event OnEndCursorOver(StaticMesh)
  (params (TouchedComponent :type Primitive%20Component%20Object%20Reference))
  (if (not (Variables|Default|GetisSelected))
    (Rendering|Material|SetMaterial (Variables|Default|GetStaticMesh) 0 (Variables|Default|GetmatBase))))

(event EventSelect
  (Variables|Default|SetisSelected true)
  (Rendering|Material|SetMaterial (Variables|Default|GetStaticMesh) 0 (Variables|Default|GetmatSelect)))

(event EventDeselect
  (Variables|Default|SetisSelected false)
  (Rendering|Material|SetMaterial (Variables|Default|GetStaticMesh) 0 (Variables|Default|GetmatBase)))

(event EventRightClick
  (params (hit :type Hit%20Result%20Structure))
  (AI|AIMoveTo self (.Location (Collision|BreakHitResult hit)) 0 5.0 false
    (:OnSuccess
      (Development|PrintText "AI move complete" true true "(R=0.000000,G=1.000000,B=0.142064,A=1.000000)"))
    (:OnFail
      (Development|PrintText "AI Couldn't reach" true true "(R=1.000000,G=0.000000,B=0.028928,A=1.000000)"))))

(fn ConstructionScript)