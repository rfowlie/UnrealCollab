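; Base selectable unit pawn that handles hover and selection feedback, right-click movement, health and allegiance.
; Cursor and select events swap mesh materials, and selection also toggles a particle effect and health bar widget.
; Right-click hits feed AI MoveTo, while damage clamps health, updates the widget and destroys the unit at zero.
; Allegiance comes from a data table row keyed by unit name, with getters exposing it and UI info.
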(event OnBeginCursorOver(StaticMesh)
  (params (TouchedComponent :type Primitive%20Component%20Object%20Reference))
  ;[1 1 1] cursor over
  (if (not (Variables|Unit|GetisSelected))
    (Rendering|Material|SetMaterial (Variables|Default|GetStaticMesh) 0 (Variables|Unit|GetmatHighlight))))

(event OnEndCursorOver(StaticMesh)
  (params (TouchedComponent :type Primitive%20Component%20Object%20Reference))
  ;[1 1 1] cursor exit
  (if (not (Variables|Unit|GetisSelected))
    (Rendering|Material|SetMaterial (Variables|Default|GetStaticMesh) 0 (Variables|Unit|GetmatBase))))

(event Custom|CustomEvent_MoveToLocation
  (params (location :type Vector))
  (AI|AIMoveTo self location 0 (Variables|AI|GetacceptanceRadiusAI) false
    (:OnSuccess
      (Development|PrintText "AI move complete" true true "(R=0.000000,G=1.000000,B=0.142064,A=1.000000)"))
    (:OnFail
      (Development|PrintText "AI Couldn't reach" true true "(R=1.000000,G=0.000000,B=0.028928,A=1.000000)"))))

(event EventBeginPlay
  ;[1 1 1] set allegiance from data table
  (CallFunction|SetAllegiance)
  ;[1 1 1] Turn off particle System
  (Components|Activation|Deactivate (Variables|Default|GetParticleSystem_Selectable))
  ;[1 1 1] Ensure health at max
  (Variables|Unit|SethealthCurrent (Variables|Unit|Gethealthmax))
  (CallFunction|UpdateHealthUI)
  (Rendering|SetVisibility (Variables|Default|GetHealthBar) false false))

(event EventDamaged
  (params (incomingDamage :type Integer))
  ;[1 1 1] Damage
  (Variables|Unit|SethealthCurrent (Math|Integer|Clamp(Integer) (- (Variables|Unit|GethealthCurrent) incomingDamage) 0 (Variables|Unit|Gethealthmax)))
  (CallFunction|UpdateHealthUI)
  (if (== (Variables|Unit|GethealthCurrent) 0)
    (Development|PrintString "Unit at zero health")
    (CallFunction|Destroyed)
    (else
      (Development|PrintString (Utilities|String|Append "Unit health: " (Utilities|String|ToString(Integer) (Variables|Unit|GethealthCurrent)))))))

(event EventDestroyed
  ;[1 1 1] Destroy
  (Actor|DestroyActor))

(event EventSelect
  ;[1 1 1] select
  (Variables|Unit|SetisSelected true)
  (Rendering|Material|SetMaterial (Variables|Default|GetStaticMesh) 0 (Variables|Unit|GetmatSelect))
  (Components|Activation|Activate (Variables|Default|GetParticleSystem_Selectable) false)
  (Rendering|SetVisibility (Variables|Default|GetHealthBar) true false))

(event EventDeselect
  ;[1 1 1] deselect
  (Variables|Unit|SetisSelected false)
  (Rendering|Material|SetMaterial (Variables|Default|GetStaticMesh) 0 (Variables|Unit|GetmatBase))
  (Components|Activation|Deactivate (Variables|Default|GetParticleSystem_Selectable))
  (Rendering|SetVisibility (Variables|Default|GetHealthBar) false false))

(event EventRightClick
  (params (hit :type Hit%20Result%20Structure))
  ;[1 1 1] right click
  (CallFunction|CustomEventMovetoLocation (.Location (Collision|BreakHitResult hit))))

(fn ConstructionScript)

(fn HealthPercentage
  (return (/ (Math|Conversions|ToFloat(Integer) (Variables|Unit|GethealthCurrent)) (Math|Conversions|ToFloat(Integer) (Variables|Unit|Gethealthmax)))))

(fn SetAllegiance
  (bind _unitname (Variables|Unit|GetunitName))
  (bind _returnvalue (Utilities|GetDataTableRow "/Game/Rob/Selectable/Data/DT_UnitInfo.DT_UnitInfo" _unitname)
    (:then
      (Variables|Unit|Setallegiance (.allegiance (Utilities|Struct|BreakUnitInfo _returnvalue))))
    (:RowNotFound
      (Development|PrintString (Utilities|String|Append "Unit Info does not contain row for  " (Utilities|String|ToString(Name) _unitname)) true true "(R=0.791667,G=0.000000,B=0.028840,A=1.000000)"))))

(fn UpdateHealthUI
  (bind _aswidget_health_bar (Utilities|Casting|CastToWidget_HealthBar (UserInterface|GetUserWidgetObject (Variables|Default|GetHealthBar))))
  (Default|SetHealth _aswidget_health_bar (Variables|Unit|GethealthCurrent) (Variables|Unit|Gethealthmax)))

(fn GetUnitAllegiance
  (return (Variables|Unit|Getallegiance)))

(fn GetUnitUI
  (bind _percentage (CallFunction|HealthPercentage))
  (return (Variables|Unit|GetunitName) _percentage))