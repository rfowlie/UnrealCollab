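; BasicRover is a selectable worker unit that hauls resources between resource nodes and storage buildings.
; Right-clicking a non-empty resource picks a storage by resource type and distance, then starts an AI move, timed gather and drop-off loop until the node is empty.
; Carried amounts live in an array indexed by resource type, feeding camera-facing Oxygen and RawMinerals labels.
; On BeginPlay it registers itself with the player controller's resource manager.
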(event Custom|CustomEvent_MoveTo
  ;[1 1 1] MoveTo
  (AI|AIMoveTo self "0, 0, 0" (Variables|!Worker|GetcurrentResource) (Variables|Default|GetacceptanceRadiusAI) false
    (:OnSuccess
      (Development|PrintText "AI move complete" true true "(R=0.000000,G=1.000000,B=0.142064,A=1.000000)")
      (CallFunction|CustomEventGather))
    (:OnFail
      (Development|PrintText "AI Couldn't reach" true true "(R=1.000000,G=0.000000,B=0.028928,A=1.000000)")
      (Variables|!Worker|SetcurrentResource 0))))

(event Custom|CustomEvent_Gather
  (bind _carriedresources (Variables|!Worker|GetCarriedResources))
  (bind _currentresourcetype (Variables|!Worker|GetcurrentResourceType))
  (bind _returnvalue (Math|Conversions|ToInteger(Byte) _currentresourcetype))
  ;[1 1 1] Gather
  (Utilities|FlowControl|Delay 1.0)
  (Development|PrintText (Utilities|Text|ToText(String) (Utilities|String|Append (Utilities|String|MakeLiteralString "Got") (Utilities|String|EnumtoString (Variables|!Worker|GetcurrentResourceType)))) true true "(R=0.000000,G=1.000000,B=0.000000,A=1.000000)" 0.5)
  (bind _numbergathered (Default|GatherResources (Variables|!Worker|GetcurrentResource)))
  (if (> _numbergathered 0)
    (Utilities|Array|SetArrayElem _carriedresources _returnvalue (+ _numbergathered (Utilities|Array|Get(acopy) _carriedresources _returnvalue)))
    (CallFunction|UpdateUI)
    (Variables|!Worker|SetcurrentCarrying (+ (Variables|!Worker|GetcurrentCarrying) _numbergathered))
    (if (< (Variables|!Worker|GetcurrentCarrying) (Variables|!Worker|GetcarryingCapacity))
      (CallFunction|CustomEventGather)
      (elif (Utilities|IsValid (Variables|!Worker|GetnearestStorage))
        (CallFunction|CustomEventMovefrom)))
    (else
      ;[1 1 1] Stop working, but return held resources
      (if (> (Variables|!Worker|GetcurrentCarrying) 0)
        (CallFunction|CustomEventMovefrom)))))

(event Custom|CustomEvent_MoveFrom
  (bind _carriedresources (Variables|!Worker|GetCarriedResources))
  ;[1 1 1] MoveFrom
  (AI|AIMoveTo self "0, 0, 0" (Variables|!Worker|GetnearestStorage) (Variables|Default|GetacceptanceRadiusAI) false
    (:OnSuccess
      (Development|PrintText "AI move complete" true true "(R=0.000000,G=1.000000,B=0.142064,A=1.000000)")
      (Default|CallDropOffResource _carriedresources)
      (for (_ _array_index) _carriedresources
        (Utilities|Array|SetArrayElem (Variables|!Worker|GetCarriedResources) _array_index 0))
      (Variables|!Worker|SetcurrentCarrying 0)
      (CallFunction|UpdateUI)
      (bind _value (Default|HasResources (Variables|!Worker|GetcurrentResource)))
      (if _value
        (CallFunction|CustomEventMoveto)
        (else
          (Variables|!Worker|SetisWorking false)
          (Variables|!Worker|SetcurrentResource 0))))
    (:OnFail
      (Development|PrintText "AI Couldn't reach" true true "(R=1.000000,G=0.000000,B=0.028928,A=1.000000)"))))

(event EventTick
  (params (DeltaSeconds :type Float%20%28single-precision%29))
  ;[1 1 1] Tick
  (CallFunction|TextFaceCamera (Variables|Default|GetOxygen))
  (CallFunction|TextFaceCamera (Variables|Default|GetRawMinerals)))

(event EventRightClick
  (params (hit :type Hit%20Result%20Structure))
  (bind (_bblockinghit _binitialoverlap _time _distance _location _impactpoint _normal _impactnormal _physmat _hitactor) (Collision|BreakHitResult hit))
  ;[1 1 1] ISelectable
  (if (< (Variables|!Worker|GetcurrentCarrying) (Variables|!Worker|GetcarryingCapacity))
    (bind _asresource_bp (Utilities|Casting|CastToResource_BP _hitactor)
      (:then
        (bind _value (Default|HasResources _asresource_bp))
        (if _value
          (bind _output_get (Variables|!Worker|SetcurrentResource _asresource_bp))
          (Variables|!Worker|SetcurrentResourceType (Variables|/Game/Rob/Selectable/Classes/NoneSelectable/Resource/Resource_BP.Resource_BP_C|GetresourceType _output_get))
          (Variables|!Worker|SetisWorking true)
          (bind _storagefound (CallFunction|FindNearestStorage))
          (if _storagefound
            (CallFunction|CustomEventMoveto))
          (else
            (Variables|!Worker|SetcurrentResource 0 :!label _label)
            (Variables|!Worker|SetisWorking false)
            (AI|AIMoveTo self _location 0 (Variables|Default|GetacceptanceRadiusAI) false
              (:OnSuccess
                (Development|PrintText "AI move complete" true true "(R=0.000000,G=1.000000,B=0.142064,A=1.000000)"))
              (:OnFail
                (Development|PrintText "AI Couldn't reach" true true "(R=1.000000,G=0.000000,B=0.028928,A=1.000000)"))))))
      (:CastFailed
        (goto _label)))))

(event EventBeginPlay
  (|CallParentFunction)
  ;[1 1 1] Reverse Subscribe Resource Manager
  (bind _asplayer_controller_selectable (Utilities|Casting|CastToPlayerController_Selectable (Game|GetPlayerController 0)))
  (Default|CustomEventSubscribe (Variables|/Game/Rob/Selectable/Player/PlayerController_Selectable.PlayerController_Selectable_C|GetManager_Resources _asplayer_controller_selectable) self)
  ;[1 1 1] Resize array match number of resources
  (bind _count (CallFunction|GetResourceTypeCount))
  (Utilities|Array|Resize (Variables|!Worker|GetCarriedResources) _count))

(fn ConstructionScript
  (|CallParentFunction))

(fn UpdateUI
  (for (_array_element _array_index) (Variables|!Worker|GetCarriedResources)
    (switch int _array_index
      (:2
        (Rendering|Components|TextRender|SetText (Variables|Default|GetOxygen) (Utilities|Text|ToText(Integer) _array_element)))
      (:3
        (Rendering|Components|TextRender|SetText (Variables|Default|GetRawMinerals) (Utilities|Text|ToText(Integer) _array_element))))))

(fn FindNearestStorage
  (bind _currentresource (Variables|!Worker|GetcurrentResource))
  (bind _returnvalue (Transformation|GetActorLocation _currentresource))
  (bind _outactors (Actor|GetAllActorsOfClass "/Game/Rob/Selectable/Classes/Selectable_Actor/Building/Building_BP.Building_BP_C"))
  (if (Utilities|IsValid (Variables|!Worker|GetnearestStorage))
    _
    (elif (> (Utilities|Array|Length _outactors) 0)
      (Variables|!Worker|SetnearestStorage (Utilities|Array|Get(acopy) _outactors))
      (else
        (Development|PrintString "There are no storages " true true "(R=0.912919,G=0.000000,B=1.000000,A=1.000000)")
        (return false))))
  (for _array_element _outactors
    (if (Utilities|Enum|Equal(Enum) (Variables|!Worker|GetcurrentResourceType) (Utilities|Struct|BreakBuildingSpecs (Variables|/Game/Rob/Selectable/Classes/Selectable_Actor/Building/Building_BP.Building_BP_C|GetbuildingSpecs _array_element)))
      (if (> (Math|Vector|VectorLength (- _returnvalue (Transformation|GetActorLocation (Variables|!Worker|GetnearestStorage)))) (Math|Vector|VectorLength (- _returnvalue (Transformation|GetActorLocation _array_element))))
        (Variables|!Worker|SetnearestStorage _array_element))))
  (if (Utilities|IsValid (Variables|!Worker|GetnearestStorage))
    (Rendering|Debug|DrawDebugPoint (Transformation|GetActorLocation (Variables|!Worker|GetnearestStorage)) 5e+01 "(R=1.000000,G=1.000000,B=1.000000,A=1.000000)" 5.0)
    (return true)
    (else
      (Development|PrintString "You don't have a storage for that resource" true true "(R=1.000000,G=0.015783,B=0.000000,A=1.000000)")
      (return false))))

(fn GetUIInfo
  (bind _percentage (CallFunction|HealthPercentage))
  (return (Variables|Default|GetunitName) _percentage))