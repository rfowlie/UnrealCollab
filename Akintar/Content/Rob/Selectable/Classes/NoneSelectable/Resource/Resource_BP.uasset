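; Resource_BP is a resource node that holds a finite total and hands out one unit per gather call.
; GatherResources decrements the total and returns 1, or 0 once empty, while HasResources reports whether any remain.
; A text label shows the remaining total, refreshed on BeginPlay and each successful gather, and turns toward the camera every tick.
; Cursor hover swaps the mesh between base and highlight materials.
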(event OnBeginCursorOver(StaticMesh)
  (params (TouchedComponent :type Primitive%20Component%20Object%20Reference))
  (Rendering|Material|SetMaterial (Variables|Default|GetStaticMesh) 0 (Variables|Default|GetmatHighlight)))

(event OnEndCursorOver(StaticMesh)
  (params (TouchedComponent :type Primitive%20Component%20Object%20Reference))
  (Rendering|Material|SetMaterial (Variables|Default|GetStaticMesh) 0 (Variables|Default|GetmatBase)))

(event EventTick
  (params (DeltaSeconds :type Float%20%28single-precision%29))
  ;[1 1 1] Tick
  (CallFunction|TextFaceCamera (Variables|Default|GetTextRender)))

(event EventBeginPlay
  ;[1 1 1] Begin
  (CallFunction|UpdateUI))

(fn ConstructionScript)

(fn GatherResources
  (if (> (Variables|Default|GetresourceTotal) 0)
    (Variables|Default|SetresourceTotal (- (Variables|Default|GetresourceTotal) 1))
    (CallFunction|UpdateUI)
    (return 1)
    (else
      (return 0))))

(fn UpdateUI
  (Rendering|Components|TextRender|SetText (Variables|Default|GetTextRender) (Utilities|Text|ToText(String) (Utilities|String|Append "Resource Total: " (Utilities|String|ToString(Text) (Utilities|Text|ToText(Integer) (Variables|Default|GetresourceTotal)))))))

(fn HasResources
  (return (> (Variables|Default|GetresourceTotal) 0)))