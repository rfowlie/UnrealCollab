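; Base Blueprint for selectable actors that show hover and selection state on a static mesh.
; Cursor-over events swap the mesh's first material between base and highlight while the actor is unselected.
; Select and Deselect events set the IsSelected flag and apply the select or base material.
; A SetStaticMesh function replaces the displayed mesh.
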(event OnBeginCursorOver(StaticMesh)
  (params (TouchedComponent :type Primitive%20Component%20Object%20Reference))
  (if (not (Variables|Default|GetisSelected))
    (Rendering|Material|SetMaterial (Variables|Default|GetStaticMesh) 0 (Variables|Default|GetmatHighlight))))

(event OnEndCursorOver(StaticMesh)
  (params (TouchedComponent :type Primitive%20Component%20Object%20Reference))
  (if (not (Variables|Default|GetisSelected))
    (Rendering|Material|SetMaterial (Variables|Default|GetStaticMesh) 0 (Variables|Default|GetmatBase))))

(event EventBeginPlay)

(event EventSelect
  (Variables|Default|SetisSelected true)
  (Rendering|Material|SetMaterial (Variables|Default|GetStaticMesh) 0 (Variables|Default|GetmatSelect)))

(event EventDeselect
  (Variables|Default|SetisSelected false)
  (Rendering|Material|SetMaterial (Variables|Default|GetStaticMesh) 0 (Variables|Default|GetmatBase)))

(fn ConstructionScript)

(fn SetStaticMesh
  (params (SM :type Static%20Mesh%20Object%20Reference))
  (Components|StaticMesh|SetStaticMesh (Variables|Default|GetStaticMesh) SM))