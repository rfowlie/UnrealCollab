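; BuildPlaceholder_BP is a placeholder actor for building that tints its mesh green for valid or red for invalid.
; BeginPlay creates a dynamic instance of M_BuildPlaceholder on the static mesh and starts it in the valid state.
; Custom events set the Colour parameter to switch validity and toggle the mesh's visibility, with no placement checks in this Blueprint.
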(event Custom|CustomEvent_Valid
  ;[1 1 1] Set Colour
  (Rendering|Material|SetVectorParameterValue (Variables|Default|GetdynMat) "Colour" "(R=0.000000,G=1.000000,B=0.000000,A=1.000000)" :!class /Script/Engine.MaterialInstanceDynamic))

(event Custom|CustomEvent_InValid
  ;[1 1 1] Set Colour
  (Rendering|Material|SetVectorParameterValue (Variables|Default|GetdynMat) "Colour" "(R=1.000000,G=0.024906,B=0.000000,A=1.000000)" :!class /Script/Engine.MaterialInstanceDynamic))

(event Custom|CustomEvent_Visible
  ;[1 1 1] Set Visibility
  (Rendering|SetVisibility (Variables|Default|GetStaticMesh) true false))

(event Custom|CustomEvent_Invisible
  ;[1 1 1] Set Visibility
  (Rendering|SetVisibility (Variables|Default|GetStaticMesh) false false))

(event EventBeginPlay
  ;[1 1 1] Dynamic Material Instance
  (bind _returnvalue (Rendering|Material|CreateDynamicMaterialInstance (Variables|Default|GetStaticMesh) 0 "/Game/Rob/Selectable/Classes/Placeholder/M_BuildPlaceholder.M_BuildPlaceholder" "None" :!class /Script/Engine.PrimitiveComponent))
  (Variables|Default|SetdynMat _returnvalue)
  (CallFunction|CustomEventValid))

(fn ConstructionScript)